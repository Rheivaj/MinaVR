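; BP_Ore is a mineable rock that a pickaxe hit has roughly a one-in-three chance of destroying.
; Its sphere overlap accepts only a BP_Pickaxe capsule, then calls DestruccionRocaMedia, which returns true when the rock survives a random roll seeded by the current millisecond.
; Survival plays a fail sound; destruction increments the score on the BP_Score actor, plays a success sound and destroys the ore.
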(event `self.Sphere.OnComponentBeginOverlap`
  (params (OverlappedComponent :type "PrimitiveComponent Object Reference") (OtherActor :type "Actor Object Reference") (OtherComp :type "PrimitiveComponent Object Reference") (OtherBodyIndex :type Integer) (bFromSweep :type Boolean) (SweepResult :type "HitResult Structure (by ref)"))
  (bind _score (`self.Score`))
  ;[1 1 1] Comprueba la colision de la esfera del mineral con la capsula del pico
  (cast `/Game/MyBlueprints/BP_Pickaxe` OtherActor)
  (cast `CapsuleComponent` OtherComp)
  (`KismetSystemLibrary.PrintString` "Colision pico/roca")
  ;[1 1 1] Funcion que devuelve un booleano(RockLife) para saber si la roca ha muerto
  (bind _rocklife (`self.DestruccionRocaMedia`))
  (if _rocklife
    ;[1 1 1] No se ha destruido la roca por tanto se reproduce el sonido de Fallo
    (`KismetSystemLibrary.PrintString` "Roca viva")
    (`GameplayStatics.SpawnSound2D` "/Game/Audio/fail_Cue.fail_Cue" 1.0 1.0 0.0 null)
    (else
      ;[1 1 1] Se ha destruido por lo que se actuliza el Score, se reproduce el sonido de exito y se destruye el mineral
      (`KismetSystemLibrary.PrintString` "Roca muerta")
      (bind _returnvalue (`GameplayStatics.GetActorOfClass` "/Game/MyBlueprints/BP_Score.BP_Score_C"))
      (set `self.Score` _returnvalue)
      (bind _result (`/Engine/EditorBlueprintResources/StandardMacros.IncrementInt` (`/Game/MyBlueprints/BP_Score.Score` _score))
        (:`  `
          (`/Game/MyBlueprints/BP_Score.SetScore` _score _result)
          (`GameplayStatics.SpawnSound2D` "/Game/Audio/success_Cue.success_Cue" 1.0 1.0 0.0 null)
          (`self.K2_DestroyActor`))))))

(fn `DestruccionRocaMedia`
  (returns (RockLife :type Boolean))
  (locals (Bool :type Boolean) (Value :type Integer))
  (bind _output_get (set `local.Value` (`KismetMathLibrary.RandomIntegerFromStream` 100 (`KismetMathLibrary.MakeRandomStream` (`KismetMathLibrary.GetMillisecond` (`KismetMathLibrary.UtcNow`))))))
  (`KismetSystemLibrary.PrintString` (`KismetStringLibrary.Conv_IntToString` _output_get))
  ;[1 1 1] Si es mayor o igual a 37 la roca sigue viva sino significa que ha muerto
  (bind _output_get_2 (set `local.Bool` (>= (`local.Value`) 37)))
  (return _output_get_2))

(fn `UserConstructionScript`)