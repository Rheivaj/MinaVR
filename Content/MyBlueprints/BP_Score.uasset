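; BP_Score is a score display that shows the current score on a TextRender and detects the win condition.
; SetScore writes the value it receives to the text and stores it in Score.
; When the score is exactly 29, it prints a victory message, plays the Win_Cue sound and spawns BP_Win just above the text.
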(fn `SetScore`
  (params (NewScore :type Integer))
  ;[1 1 1] Funcion que pone el TextRender y Score al valor que se le pasa por parametro
  (`TextRenderComponent.K2_SetText` (`self.TextRender`) (`KismetTextLibrary.Conv_IntToText` NewScore))
  ;[1 1 1] Comprueba si la puntuacion es mayor a 28(Victoria)
  (bind _output_get (set `self.Score` NewScore))
  (if (== _output_get 29)
    (`KismetSystemLibrary.PrintString` "ERES UN LOCO DEL PICO")
    (`GameplayStatics.PlaySound2D` "/Game/Audio/win_Cue.win_Cue" 1.0 1.0 0.0 null null)
    (`|SpawnActorFromClass` "/Game/MyBlueprints/BP_Win.BP_Win_C" (`KismetMathLibrary.Conv_VectorToTransform` (+ (`SceneComponent.GetSocketLocation` (`self.TextRender`) "None") (0.0 0.0 10.0))) "Undefined" "OverrideRootScale" null null)))

(fn `UserConstructionScript`)